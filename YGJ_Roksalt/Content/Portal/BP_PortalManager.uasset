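; Manager for a linked portal pair that keeps each portal's view component matched to the player's camera.
; Every Tick, two mirrored updaters map the player camera's world location and rotation from one portal's frame into the other's, then move that destination portal's PortalView there.
; The mapping uses the rotation delta between the portal roots, with the destination's yaw turned 180 degrees.
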(event EventTick
  (params (DeltaSeconds :type Float%20%28single-precision%29))
  (CallFunction|Portal1Updater)
  (CallFunction|Portal2Updater))

(fn ConstructionScript)

(fn Portal1Updater
  (bind _returnvalue (Game|GetPlayerCameraManager 0))
  (bind _portal1 (Variables|Default|GetPortal1))
  (bind _portal2 (Variables|Default|GetPortal2))
  (bind _defaultsceneroot (Variables|/Game/Portal/BP_Portal2.BP_Portal2_C|GetDefaultSceneRoot _portal2))
  (bind _defaultsceneroot_2 (Variables|/Game/Portal/BP_Portal1.BP_Portal1_C|GetDefaultSceneRoot _portal1))
  (bind _transformcomponent (Variables|/Script/Engine.PlayerCameraManager|GetTransformComponent _returnvalue))
  (bind _returnvalue_2 (Transformation|GetWorldRotation _defaultsceneroot_2))
  (bind _returnvalue_3 (Transformation|GetWorldRotation _defaultsceneroot))
  (bind _returnvalue_4 (Transformation|GetWorldRotation _transformcomponent))
  (bind _returnvalue_5 (- (.yaw _returnvalue_3) 1.8e+02))
  (bind _returnvalue_6 (Math|Rotator|MakeRotator (.roll _returnvalue_3) (.pitch _returnvalue_3) _returnvalue_5))
  (bind _returnvalue_7 (Math|Rotator|Delta(Rotator) _returnvalue_6 _returnvalue_2))
  (bind _returnvalue_8 (Math|Rotator|CombineRotators _returnvalue_4 _returnvalue_7))
  (Variables|Default|SetPortal1Rotator _returnvalue_8)
  (Transformation|SetWorldLocationAndRotation (Variables|/Game/Portal/BP_Portal2.BP_Portal2_C|GetPortalView (Variables|Default|GetPortal2)) (+ (- (Transformation|GetWorldLocation _defaultsceneroot) (Math|Vector|RotateVector (Transformation|GetWorldLocation _defaultsceneroot_2) _returnvalue_7)) (Math|Vector|RotateVector (Transformation|GetWorldLocation _transformcomponent) _returnvalue_7)) _returnvalue_8 false false))

(fn Portal2Updater
  (bind _returnvalue (Game|GetPlayerCameraManager 0))
  (bind _portal1 (Variables|Default|GetPortal1))
  (bind _portal2 (Variables|Default|GetPortal2))
  (bind _defaultsceneroot (Variables|/Game/Portal/BP_Portal2.BP_Portal2_C|GetDefaultSceneRoot _portal2))
  (bind _defaultsceneroot_2 (Variables|/Game/Portal/BP_Portal1.BP_Portal1_C|GetDefaultSceneRoot _portal1))
  (bind _transformcomponent (Variables|/Script/Engine.PlayerCameraManager|GetTransformComponent _returnvalue))
  (bind _returnvalue_2 (Transformation|GetWorldRotation _defaultsceneroot))
  (bind _returnvalue_3 (Transformation|GetWorldRotation _defaultsceneroot_2))
  (bind _returnvalue_4 (Transformation|GetWorldRotation _transformcomponent))
  (bind _returnvalue_5 (- (.yaw _returnvalue_3) 1.8e+02))
  (bind _returnvalue_6 (Math|Rotator|MakeRotator (.roll _returnvalue_3) (.pitch _returnvalue_3) _returnvalue_5))
  (bind _returnvalue_7 (Math|Rotator|Delta(Rotator) _returnvalue_6 _returnvalue_2))
  (bind _returnvalue_8 (Math|Rotator|CombineRotators _returnvalue_4 _returnvalue_7))
  (Variables|Default|SetPortal2Rotator _returnvalue_8)
  (Transformation|SetWorldLocationAndRotation (Variables|/Game/Portal/BP_Portal1.BP_Portal1_C|GetPortalView (Variables|Default|GetPortal1)) (+ (- (Transformation|GetWorldLocation _defaultsceneroot_2) (Math|Vector|RotateVector (Transformation|GetWorldLocation _defaultsceneroot) _returnvalue_7)) (Math|Vector|RotateVector (Transformation|GetWorldLocation _transformcomponent) _returnvalue_7)) _returnvalue_8 false false))