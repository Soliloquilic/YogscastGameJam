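; BP_Portal1 is a portal actor that teleports the first-person player to Portal2 when its Portal component is overlapped.
; The player's PortalManager supplies the destination, the Portal1Rotator applied as control rotation, and a shared CanTeleport flag.
; That flag blocks re-triggering until a half-second delay ends.
; It is cleared before the character cast, so overlap by another actor type leaves it false.
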(event OnComponentBeginOverlap(Portal)
  (params (OverlappedComponent :type Primitive%20Component%20Object%20Reference) (OtherActor :type Actor%20Object%20Reference) (OtherComp :type Primitive%20Component%20Object%20Reference) (OtherBodyIndex :type Integer) (bFromSweep :type Boolean) (SweepResult :type Hit%20Result%20Structure%20%28by%20ref%29))
  (bind _playerref (Variables|Default|GetPlayerRef))
  (bind _portalmanager (Variables|/Game/FirstPersonBP/Blueprints/FirstPersonCharacter.FirstPersonCharacter_C|GetPortalManager _playerref))
  (if (Variables|/Game/Portal/BP_PortalManager.BP_PortalManager_C|GetCanTeleport _portalmanager)
    (Variables|/Game/Portal/BP_PortalManager.BP_PortalManager_C|SetCanTeleport _portalmanager false)
    (bind _asfirst_person_character (Utilities|Casting|CastToFirstPersonCharacter OtherActor))
    (Pawn|SetControlRotation (Game|GetPlayerController 0) (Variables|/Game/Portal/BP_PortalManager.BP_PortalManager_C|GetPortal1Rotator (Variables|/Game/FirstPersonBP/Blueprints/FirstPersonCharacter.FirstPersonCharacter_C|GetPortalManager _asfirst_person_character)))
    (Transformation|SetActorLocationAndRotation _asfirst_person_character (Transformation|GetWorldLocation (Variables|/Game/Portal/BP_Portal2.BP_Portal2_C|GetDefaultSceneRoot (Variables|/Game/Portal/BP_PortalManager.BP_PortalManager_C|GetPortal2 (Variables|/Game/FirstPersonBP/Blueprints/FirstPersonCharacter.FirstPersonCharacter_C|GetPortalManager _asfirst_person_character)))) "0.0,0.0,0.0")
    (Utilities|FlowControl|Delay 0.5)
    (Variables|/Game/Portal/BP_PortalManager.BP_PortalManager_C|SetCanTeleport (Variables|/Game/FirstPersonBP/Blueprints/FirstPersonCharacter.FirstPersonCharacter_C|GetPortalManager (Variables|Default|GetPlayerRef)) true)))

(event EventBeginPlay
  (bind _asfirst_person_character (Utilities|Casting|CastToFirstPersonCharacter (Game|GetPlayerCharacter 0)))
  (Variables|Default|SetPlayerRef _asfirst_person_character))

(fn ConstructionScript)